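; Behavior tree task that closes out an enemy's attack sequence.
; It clears the should-attack blackboard flag and hands the attack token back to the AI Director stored on the blackboard.
; It then tells the Gladiator AI controller to end its attack sequence and succeeds, or fails with a debug message if no director is found.
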(event `self.ReceiveExecuteAI`
  (params (OwnerController :type "AIController Object Reference") (ControlledPawn :type "Pawn Object Reference"))
  (set `self.Owner Controller` OwnerController)
  (bind _output_get (set `self.Blackboard` (`AIController.Blackboard` OwnerController)))
  (`BlackboardComponent.SetValueAsBool` _output_get (`self.ShouldAttackKey`) false)
  (bind _asaidirector (cast `AIDirector` (`BlackboardComponent.GetValueAsObject` (`self.Blackboard`) (`self.DirectorKey`)))
    (:`then`
      (`AIDirector.ReturnAttackToken` _asaidirector)
      (bind _asaic_gladiator (cast `/Game/Blueprints/Enemy/AIC_Gladiator` (`self.Owner Controller`)))
      (`GladiatorAIController.EndAttackSequence` _asaic_gladiator)
      (`self.FinishExecute` true))
    (:`CastFailed`
      (`KismetSystemLibrary.PrintString` "No AI Director found" true true (struct :`R` 1.0 :`A` 1.0) 10.0)
      (`self.FinishExecute` false))))