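; BP_EnemyGladiator is an enemy Blueprint that keeps its life bar in sync when it takes damage.
; On UpdateDamage, it relies on the parent class to have already changed the Life component's value.
; It then writes the current-to-max life ratio into the WBP_EnemyLife widget of its LifeBar and prints the current life as debug text.
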(event `self.UpdateDamage`
  (bind _life (`self.Life`))
  ;[1 0.1867 0] Parent class already updated life. We only need to update the display here
  (bind _aswbp_enemy_life (cast `/Game/Blueprints/Enemy/WBP_EnemyLife` (`WidgetComponent.GetWidget` (`self.LifeBar`))))
  (bind _returnvalue (`LifeComponent.GetLife` _life))
  (set `GladiatorLifeWidget.LifeRatio` (/ _returnvalue (`LifeComponent.MaxLife` _life)) _aswbp_enemy_life)
  (`KismetSystemLibrary.PrintString` (`KismetStringLibrary.Concat_StrStr` "current life : " (`KismetStringLibrary.Conv_DoubleToString` _returnvalue)) true true (struct :`R` 1.0 :`G` 0.539098 :`B` 0.163319 :`A` 1.0)))

(fn `UserConstructionScript`)