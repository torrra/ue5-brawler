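; Anim notify state that plays surface-specific footstep sounds during animations.
; On notify begin, it runs a Visibility line trace from the owning actor's location 200 units along its down vector.
; A hit's physical surface selects the Sand or Stone sound, and other surfaces stay silent.
; The sound's location is only the down-offset vector, without the actor's location added, so it plays near world origin.
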(fn `Received_NotifyBegin`
  (params (MeshComp :type "SkeletalMeshComponent Object Reference") (Animation :type "AnimSequenceBase Object Reference") (TotalDuration :type "Float (single-precision)") (EventReference :type "AnimNotifyEventReference Structure (by ref)"))
  (returns (ReturnValue :type Boolean))
  (locals (OwnerActor :type "Actor Object Reference"))
  (bind _returnvalue (`ActorComponent.GetOwner` MeshComp))
  (bind _returnvalue_2 (`Actor.K2_GetActorLocation` _returnvalue))
  (bind _returnvalue_3 (* (`Actor.GetActorUpVector` _returnvalue) -200.0))
  (bind _output_get (set `local.OwnerActor` _returnvalue))
  (bind (_outhit _returnvalue_4) (`KismetSystemLibrary.LineTraceSingle` _output_get _returnvalue_2 (+ _returnvalue_2 _returnvalue_3) "TraceTypeQuery1"))
  (if _returnvalue_4
    (switch `EPhysicalSurface` (`GameplayStatics.GetSurfaceType` _outhit)
      (:`SurfaceType_Default`
        _)
      (:`SurfaceType1`
        (`GameplayStatics.PlaySoundAtLocation` (`local.OwnerActor`) "/Game/Sounds/Characters/Footsteps/MS_Sand.MS_Sand" _returnvalue_3 (struct) 1.0 1.0 0.0 null null null null))
      (:`SurfaceType2`
        (`GameplayStatics.PlaySoundAtLocation` (`local.OwnerActor`) "/Game/Sounds/Characters/Footsteps/MS_Stone.MS_Stone" _returnvalue_3 (struct) 1.0 1.0 0.0 null null null null)))
    (return true)))